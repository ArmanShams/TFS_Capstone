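; HUD Blueprint that draws a custom mouse cursor for the first player controller.
; Each DrawHUD call renders the MAT_Cursor material as a small fixed-size square centered on the mouse position.
; It shifts the position by half the difference between the HUD draw size and the viewport size to compensate when the two differ.
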(event EventDrawHUD
  (params (SizeX :type Integer) (SizeY :type Integer))
  (bind _returnvalue (Math|Float|MakeLiteralFloat 32.0))
  (bind _returnvalue_2 (Game|GetPlayerController 0))
  (bind _returnvalue_3 (/ _returnvalue 2.0))
  (bind (_locationx _locationy) (Game|Player|GetMousePosition _returnvalue_2))
  (bind (_sizex _sizey) (HUD|GetViewportSize _returnvalue_2))
  (Canvas|DrawMaterial "/Game/Materials/MAT_Cursor.MAT_Cursor" (- (+ (/ (Math|Conversions|ToFloat(Integer) (- SizeX _sizex)) 2.0) _locationx) _returnvalue_3) (- (+ _locationy (/ (Math|Conversions|ToFloat(Integer) (- SizeY _sizey)) 2.0)) _returnvalue_3) _returnvalue _returnvalue 0.0 0.0 1.0 1.0))

(fn ConstructionScript)