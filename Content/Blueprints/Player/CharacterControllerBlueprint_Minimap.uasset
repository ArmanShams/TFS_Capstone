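; Player character Blueprint that handles form-based screen effects, startup music and the pause menu for a human/wolf shapeshifter.
; Tick maps CurrentForm to WolfVision and DeathVision in the WolfParams material collection, repeatedly spawning delayed blood splatter while dead.
; Escape, P and focus loss while alive share the pause path, which reuses one menu widget and manages cursor and input.
; Hard-CC stars logic is unconnected, and no minimap logic appears despite the name.
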(event EventOnDamageTaken)

(event EventOnGameFocusLost
  (bind _returnvalue (Game|GetPlayerController 0))
  (bind _returnvalue_2 (Game|GetPlayerController 0))
  (if (Utilities|Enum|NotEqual(Enum) (Variables|Default|GetCurrentForm) "DEAD")
    (if (not (Game|IsGamePaused))
      (Variables|/Script/Engine.PlayerController|SetbShowMouseCursor _returnvalue_2 true)
      (Variables|/Script/Engine.PlayerController|SetCurrentMouseCursor _returnvalue_2 "Default")
      (Variables|/Script/Engine.PlayerController|SetbShowMouseCursor _returnvalue true)
      (Variables|/Script/Engine.PlayerController|SetCurrentMouseCursor _returnvalue "Default")
      (if (Utilities|IsValid (Variables|Default|GetPauseMenuReference))
        _
        (else
          (bind _returnvalue_3 (UserInterface|CreateWidget "/Game/Blueprints/PauseMenuWidget.PauseMenuWidget_C" _returnvalue))
          (Variables|Default|SetPauseMenuReference _returnvalue_3)))
      (UserInterface|Viewport|AddtoViewport (Variables|Default|GetPauseMenuReference) 400)
      (Input|SetInputModeUIOnly _returnvalue (Variables|Default|GetPauseMenuReference) "DoNotLock")
      (Game|SetGamePaused true))))

(event EventBeginPlay
  (Audio|SpawnSound2D "/Game/Audio/Music/A_MUS_CombatDrums.A_MUS_CombatDrums" 1.0 1.0 0.0)
  (Audio|SpawnSound2D "/Game/Audio/Music/A_MUS_Ambience.A_MUS_Ambience" 0.3 1.0 0.0)
  (Variables|/Script/Engine.PlayerController|SetbShowMouseCursor (Game|GetPlayerController 0) false))

(event EventOnDeath
  (bind _returnvalue (Game|GetPlayerController 0))
  (Variables|/Script/Engine.PlayerController|SetCurrentMouseCursor _returnvalue "Default")
  (Variables|/Script/Engine.PlayerController|SetbShowMouseCursor _returnvalue true))

(event EventTick
  (params (DeltaSeconds :type Float%20%28single-precision%29))
  (Utilities|FlowControl|Sequence
    (:then_0
      (switch Utilities|FlowControl|Switch|SwitchonTransformationState (Variables|Default|GetCurrentForm)
        (:DEAD
          (Utilities|FlowControl|Delay 0.2)
          (Effects|SpawnEmitterAttached "/Game/FX/BloodSplatter/PS_BloodSplatter.PS_BloodSplatter" (Variables|Character|GetMesh) "None")
          (Rendering|Material|SetScalarParameterValue "/Game/FX/WolfParams.WolfParams" "DeathVision" 1.0 :!class /Script/Engine.KismetMaterialLibrary)
          (Rendering|Material|SetScalarParameterValue "/Game/FX/WolfParams.WolfParams" "WolfVision" 0.0 :!class /Script/Engine.KismetMaterialLibrary))
        (:HUMAN
          (Rendering|Material|SetScalarParameterValue "/Game/FX/WolfParams.WolfParams" "WolfVision" 0.0 :!class /Script/Engine.KismetMaterialLibrary)
          (Rendering|Material|SetScalarParameterValue "/Game/FX/WolfParams.WolfParams" "DeathVision" 0.0 :!class /Script/Engine.KismetMaterialLibrary))
        (:WOLF
          (Rendering|Material|SetScalarParameterValue "/Game/FX/WolfParams.WolfParams" "WolfVision" 1.0 :!class /Script/Engine.KismetMaterialLibrary)
          (Rendering|Material|SetScalarParameterValue "/Game/FX/WolfParams.WolfParams" "DeathVision" 0.0 :!class /Script/Engine.KismetMaterialLibrary))))))

(event Input|KeyboardEvents|Escape
  (params (Key :type Key%20Structure :default "AnyKey"))
  (bind _returnvalue (Game|GetPlayerController 0))
  (:Pressed
    (if (Game|IsGamePaused)
      (Variables|/Script/Engine.PlayerController|SetbShowMouseCursor _returnvalue false)
      (Widget|RemovefromParent (Variables|Default|GetPauseMenuReference))
      (Class|Widget|SetUserFocus (Variables|Default|GetInGameHud) _returnvalue)
      (Game|SetGamePaused false)
      (else
        (Variables|/Script/Engine.PlayerController|SetbShowMouseCursor _returnvalue true)
        (Variables|/Script/Engine.PlayerController|SetCurrentMouseCursor _returnvalue "Default")
        (if (Utilities|IsValid (Variables|Default|GetPauseMenuReference))
          _
          (else
            (bind _returnvalue_2 (UserInterface|CreateWidget "/Game/Blueprints/PauseMenuWidget.PauseMenuWidget_C" _returnvalue))
            (Variables|Default|SetPauseMenuReference _returnvalue_2)))
        (UserInterface|Viewport|AddtoViewport (Variables|Default|GetPauseMenuReference) 400)
        (Input|SetInputModeUIOnly _returnvalue (Variables|Default|GetPauseMenuReference) "DoNotLock")
        (Game|SetGamePaused true)))))

(event Input|KeyboardEvents|P
  (params (Key :type Key%20Structure :default "AnyKey"))
  (bind _returnvalue (Game|GetPlayerController 0))
  (:Pressed
    (if (Game|IsGamePaused)
      (Variables|/Script/Engine.PlayerController|SetbShowMouseCursor _returnvalue false)
      (Widget|RemovefromParent (Variables|Default|GetPauseMenuReference))
      (Class|Widget|SetUserFocus (Variables|Default|GetInGameHud) _returnvalue)
      (Game|SetGamePaused false)
      (else
        (Variables|/Script/Engine.PlayerController|SetbShowMouseCursor _returnvalue true)
        (Variables|/Script/Engine.PlayerController|SetCurrentMouseCursor _returnvalue "Default")
        (if (Utilities|IsValid (Variables|Default|GetPauseMenuReference))
          _
          (else
            (bind _returnvalue_2 (UserInterface|CreateWidget "/Game/Blueprints/PauseMenuWidget.PauseMenuWidget_C" _returnvalue))
            (Variables|Default|SetPauseMenuReference _returnvalue_2)))
        (UserInterface|Viewport|AddtoViewport (Variables|Default|GetPauseMenuReference) 400)
        (Input|SetInputModeUIOnly _returnvalue (Variables|Default|GetPauseMenuReference) "DoNotLock")
        (Game|SetGamePaused true)))))

(fn ConstructionScript)