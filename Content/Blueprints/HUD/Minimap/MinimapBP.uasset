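; MinimapBP is a minimap Blueprint that drives the player icon for the pause map.
; On BeginPlay it moves its PositioningTool component to the world origin to center the map.
; Every Tick it moves the player icon sprite to the player character's X and Y at a fixed height.
; An unconnected debug sequence for printing the pause minimap's location never runs.
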(event EventBeginPlay
  ;[1 1 1] Centers the minimap
  (Transformation|SetWorldLocation (Variables|Default|GetPositioningTool) (Math|Vector|MakeVector 0.0 0.0 0.0) false false))

(event EventTick
  (params (DeltaSeconds :type Float%20%28single-precision%29))
  (bind _returnvalue (Game|GetPlayerCharacter 0))
  (bind _returnvalue_2 (Transformation|GetActorLocation _returnvalue))
  (bind (_x _y) (Math|Vector|BreakVector _returnvalue_2))
  (Transformation|SetWorldLocation (Variables|Default|GetSpirte_PlayerIconForPauseMap) (Math|Vector|MakeVector _x _y 23.2) false false))

(fn ConstructionScript)