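; Elevator actor that lowers its cage while the player pawn overlaps TriggerVolume, until the cage passes a fixed world-height limit, with no return trip.
; Tick, gated by a short Delay, steps the cage down, the counterweight up and the wheel axis around in roll.
; Half-alpha lerps toward fixed offsets yield constant increments without delta-time scaling.
; Any overlap beginning on the trigger sets CageCollision to block GameTraceChannel1.
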(event OnComponentBeginOverlap(TriggerVolume)
  (params (OverlappedComponent :type Primitive%20Component%20Object%20Reference) (OtherActor :type Actor%20Object%20Reference) (OtherComp :type Primitive%20Component%20Object%20Reference) (OtherBodyIndex :type Integer) (bFromSweep :type Boolean) (SweepResult :type Hit%20Result%20Structure%20%28by%20ref%29))
  (Collision|SetCollisionResponsetoChannel (Variables|Default|GetCageCollision) "ECC_GameTraceChannel1" "ECR_Block"))

(event EventTick
  (params (DeltaSeconds :type Float%20%28single-precision%29))
  (bind _cage (Variables|Default|GetCage))
  (bind _counterweight (Variables|Default|GetCounterWeight))
  (bind _wheelrotationaxis (Variables|Default|GetWheelRotationAxis))
  (bind _returnvalue (Transformation|GetWorldLocation _cage))
  (bind _returnvalue_2 (Transformation|GetWorldLocation _counterweight))
  (bind _returnvalue_3 (Transformation|GetWorldRotation _wheelrotationaxis))
  (bind (_roll _pitch _yaw) (Math|Rotator|BreakRotator _returnvalue_3))
  (if (Collision|IsOverlappingActor (Variables|Default|GetTriggerVolume) (Game|Player|GetPlayerPawn 0) :!class /Script/Engine.PrimitiveComponent)
    (Utilities|FlowControl|Delay 0.01)
    (if (>= (.Z (Math|Vector|BreakVector (Transformation|GetWorldLocation (Variables|Default|GetCage)))) -1.5e+03)
      (Transformation|SetWorldLocation _cage (Math|Vector|Lerp(Vector) _returnvalue (+ _returnvalue "0,0.000000,-10.000000") 0.5) false false)
      (Transformation|SetWorldLocation _counterweight (Math|Vector|Lerp(Vector) _returnvalue_2 (+ _returnvalue_2 "0, 0,10.000000") 0.5) false false)
      (Transformation|SetRelativeRotation _wheelrotationaxis (Math|Rotator|MakeRotator (Math|Float|Lerp _roll (+ _roll 5.0) 0.5) _pitch _yaw) false false))))

(fn ConstructionScript)