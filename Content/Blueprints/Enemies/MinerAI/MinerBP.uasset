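; Miner enemy Blueprint that drives its health bar, stun effect and enemy icon from Tick.
; The health bar widget receives the current health percent and is hidden when health is nearly full or nearly empty.
; During hard crowd control, scaled-up BPStars spawn above the mesh after an animation catch-up delay, guarded by a flag and destroyed afterwards.
; The enemy icon sprite follows in X and Y at a fixed world height.
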(event EventTick
  (params (DeltaSeconds :type Float%20%28single-precision%29))
  (bind _mesh (Variables|Character|GetMesh))
  (bind _healthbarwidget (Variables|Default|GetHealthBarWidget))
  (bind _sprite_enemyicon (Variables|Default|GetSprite_EnemyIcon))
  (bind _returnvalue (Transformation|GetWorldTransform _mesh))
  (bind _returnvalue_2 (Transformation|GetWorldLocation _sprite_enemyicon))
  (bind _returnvalue_3 (UserInterface|GetUserWidgetObject _healthbarwidget))
  (bind (_location _rotation _scale) (Math|Transform|BreakTransform _returnvalue))
  (bind (_x _y) (Math|Vector|BreakVector _returnvalue_2))
  (Utilities|FlowControl|Sequence
    (:then_0
      (bind _asenemy_health_bar_widget (Utilities|Casting|CastToEnemyHealthBarWidget _returnvalue_3))
      (bind _returnvalue_4 (Class|Enemy|GetHealthPercent))
      (if (or (> _returnvalue_4 0.99) (< _returnvalue_4 0.1))
        (Widget|SetVisibility _returnvalue_3 "Hidden")
        (else
          (Widget|SetVisibility _returnvalue_3 "Visible")))
      (Variables|/Game/Blueprints/Enemies/EnemyHealthBarWidget.EnemyHealthBarWidget_C|SetOwningEnemyHealthPercent _asenemy_health_bar_widget _returnvalue_4))
    (:then_1
      (if (Variables|Default|GetbIsInHardCC)
        (if (not (Variables|Default|GetParticleSystemAlive?))
          ;[1 1 1] Delay for Animation to catch up
          (Utilities|FlowControl|Delay 0.8)
          (bind _returnvalue_5 (Game|SpawnActorfromClass "/Game/FX/Stars/BPStars.BPStars_C" (Math|Transform|MakeTransform (+ _location "0, 0,200.000000") _rotation (* _scale 4)) "Undefined" 0 0))
          (Variables|Default|SetParticleSystemAlive? true))
        (elif (Variables|Default|GetParticleSystemAlive?)
          (Actor|DestroyActor _returnvalue_5)
          (Variables|Default|SetParticleSystemAlive? false))))
    (:then_2
      (Transformation|SetWorldLocation (Variables|Default|GetSprite_EnemyIcon) (Math|Vector|MakeVector _x _y 3.5e+03) false false))))

(fn ConstructionScript)