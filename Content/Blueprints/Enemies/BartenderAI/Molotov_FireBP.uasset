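; Molotov fire actor for the Bartender AI enemy that creates a temporary patch of fire where it spawns.
; On BeginPlay it plays the Molotov sound and spawns a BP_Fire at its SphereCollider's transform with enlarged scale.
; After a timed delay it shrinks the fire, then destroys it shortly after, leaving its own actor in place.
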(event EventBeginPlay
  (bind _spherecollider (Variables|Default|GetSphereCollider))
  (bind _returnvalue (Transformation|GetWorldTransform _spherecollider))
  (bind (_location _rotation _scale) (Math|Transform|BreakTransform _returnvalue))
  (Audio|SpawnSoundatLocation "/Game/Audio/SFX/A_SFX_Molotov_Cue.A_SFX_Molotov_Cue" _location)
  (bind _returnvalue_2 (Game|SpawnActorfromClass "/Game/FX/FloorFire/BP_Fire.BP_Fire_C" (Math|Transform|MakeTransform _location _rotation (+ _scale "0.500000,0.500000,0.500000")) "Undefined" 0 0))
  (Utilities|FlowControl|Delay 8.0)
  (Transformation|SetActorScale3D _returnvalue_2 "0.400000,0.400000,0.400000")
  (Utilities|FlowControl|Delay 1.0)
  (Actor|DestroyActor _returnvalue_2))

(fn ConstructionScript)