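; Railroad actor that lays modular rail track along a spline at construction time; its event graph has no active logic.
; The construction script adds colliding static meshes at fixed spacing, oriented to the spline, using straight or 45-degree pieces according to the TurningPoint flag.
; StartsInTerminal and EndsInTerminal choose end-cap pieces, with the start cap yawed 180 degrees; a non-terminal end gets another straight piece.
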(event EventBeginPlay)

(event Collision|EventActorBeginOverlap
  (params (OtherActor :type Actor%20Object%20Reference)))

(event EventTick
  (params (DeltaSeconds :type Float%20%28single-precision%29)))

(fn ConstructionScript
  (bind _splinecomponent (Variables|Default|GetSplineComponent))
  (bind _spacing (Variables|Default|GetSpacing))
  (if (Variables|Default|GetStartsInTerminal?)
    (Variables|Default|SetStartIndex 1)
    (bind _returnvalue (AddComponent|AddStaticMeshComponent false (Math|Transform|MakeTransform (.Location (Math|Transform|BreakTransform (Math|Transform|MakeTransform (Spline|GetLocationatDistanceAlongSpline _splinecomponent (* (stale _index) _spacing) "Local") (Spline|GetRotationatDistanceAlongSpline _splinecomponent (* (stale _index) _spacing) "Local")))) (Math|Rotator|MakeRotator (.Roll (Math|Rotator|BreakRotator (.Rotation (Math|Transform|BreakTransform (Math|Transform|MakeTransform (Spline|GetLocationatDistanceAlongSpline _splinecomponent (* (stale _index) _spacing) "Local") (Spline|GetRotationatDistanceAlongSpline _splinecomponent (* (stale _index) _spacing) "Local")))))) (.Pitch (Math|Rotator|BreakRotator (.Rotation (Math|Transform|BreakTransform (Math|Transform|MakeTransform (Spline|GetLocationatDistanceAlongSpline _splinecomponent (* (stale _index) _spacing) "Local") (Spline|GetRotationatDistanceAlongSpline _splinecomponent (* (stale _index) _spacing) "Local")))))) (+ (.Yaw (Math|Rotator|BreakRotator (.Rotation (Math|Transform|BreakTransform (Math|Transform|MakeTransform (Spline|GetLocationatDistanceAlongSpline _splinecomponent (* (stale _index) _spacing) "Local") (Spline|GetRotationatDistanceAlongSpline _splinecomponent (* (stale _index) _spacing) "Local")))))) 1.8e+02)) (.Scale (Math|Transform|BreakTransform (Math|Transform|MakeTransform (Spline|GetLocationatDistanceAlongSpline _splinecomponent (* (stale _index) _spacing) "Local") (Spline|GetRotationatDistanceAlongSpline _splinecomponent (* (stale _index) _spacing) "Local")))))))
    (Collision|SetCollisionEnabled _returnvalue "QueryAndPhysics")
    (Components|StaticMesh|SetStaticMesh _returnvalue "/Game/Geometry/World/M_Rail_End.M_Rail_End")
    (Rendering|Material|SetMaterial _returnvalue 0 "/Game/Materials/MI_RailTerminal.MI_RailTerminal")
    (Variables|Default|SetCurrentPointIndex (+ (Variables|Default|GetCurrentPointIndex) 1))
    (else
      (Variables|Default|SetStartIndex 0)))
  (for _index (range (Variables|Default|GetStartIndex) (- (.ReturnValue (Math|Float|Division(WholeandRemainder) (Spline|GetSplineLength (Variables|Default|GetSplineComponent)) _spacing)) 1))
    (if (Variables|Default|GetTurningPoint?)
      (bind _returnvalue_2 (AddComponent|AddStaticMeshComponent false (Math|Transform|MakeTransform (Spline|GetLocationatDistanceAlongSpline _splinecomponent (* _index _spacing) "Local") (Spline|GetRotationatDistanceAlongSpline _splinecomponent (* _index _spacing) "Local"))))
      (Collision|SetCollisionEnabled _returnvalue_2 "QueryAndPhysics")
      (Components|StaticMesh|SetStaticMesh _returnvalue_2 "/Game/Geometry/World/M_Rail_45.M_Rail_45")
      (Rendering|Material|SetMaterial _returnvalue_2 0 "/Game/Materials/MI_Rail45.MI_Rail45")
      (Variables|Default|SetCurrentPointIndex (+ (Variables|Default|GetCurrentPointIndex) 1))
      (else
        (bind _returnvalue_3 (AddComponent|AddStaticMeshComponent false (Math|Transform|MakeTransform (Spline|GetLocationatDistanceAlongSpline _splinecomponent (* _index _spacing) "Local") (Spline|GetRotationatDistanceAlongSpline _splinecomponent (* _index _spacing) "Local"))))
        (Collision|SetCollisionEnabled _returnvalue_3 "QueryAndPhysics")
        (Components|StaticMesh|SetStaticMesh _returnvalue_3 "/Game/Geometry/World/M_Rail_Straight.M_Rail_Straight")
        (Rendering|Material|SetMaterial _returnvalue_3 0 "/Game/Materials/MI_RailStraight.MI_RailStraight")
        (Variables|Default|SetCurrentPointIndex (+ (Variables|Default|GetCurrentPointIndex) 1)))))
  (if (Variables|Default|GetEndsInTerminal?)
    (bind _returnvalue_4 (AddComponent|AddStaticMeshComponent false (Math|Transform|MakeTransform (Spline|GetLocationatDistanceAlongSpline _splinecomponent (* _index _spacing) "Local") (Spline|GetRotationatDistanceAlongSpline _splinecomponent (* _index _spacing) "Local"))))
    (Collision|SetCollisionEnabled _returnvalue_4 "QueryAndPhysics")
    (Components|StaticMesh|SetStaticMesh _returnvalue_4 "/Game/Geometry/World/M_Rail_End.M_Rail_End")
    (Rendering|Material|SetMaterial _returnvalue_4 0 "/Game/Materials/MI_RailTerminal.MI_RailTerminal")
    (Variables|Default|SetCurrentPointIndex (+ (Variables|Default|GetCurrentPointIndex) 1))
    (else
      (bind _returnvalue_5 (AddComponent|AddStaticMeshComponent false (Math|Transform|MakeTransform (Spline|GetLocationatDistanceAlongSpline _splinecomponent (* _index _spacing) "Local") (Spline|GetRotationatDistanceAlongSpline _splinecomponent (* _index _spacing) "Local"))))
      (Collision|SetCollisionEnabled _returnvalue_5 "QueryAndPhysics")
      (Components|StaticMesh|SetStaticMesh _returnvalue_5 "/Game/Geometry/World/M_Rail_Straight.M_Rail_Straight")
      (Rendering|Material|SetMaterial _returnvalue_5 0 "/Game/Materials/MI_RailStraight.MI_RailStraight")
      (Variables|Default|SetCurrentPointIndex (+ (Variables|Default|GetCurrentPointIndex) 1)))))