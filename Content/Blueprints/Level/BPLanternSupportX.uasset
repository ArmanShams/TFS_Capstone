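; BPLanternSupportX is a level prop Blueprint for a lantern support with up to four lanterns, each paired with a light.
; The construction script shows or hides each lantern and its light together from a per-lamp visibility variable, propagating the change to child components.
; It has no runtime logic, as the event graph holds only disabled default events.
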(event EventBeginPlay)

(event Collision|EventActorBeginOverlap
  (params (OtherActor :type Actor%20Object%20Reference)))

(event EventTick
  (params (DeltaSeconds :type Float%20%28single-precision%29)))

(fn ConstructionScript
  (Rendering|SetVisibility (Variables|Default|GetLantern1) (Variables|Default|GetLampAVisibility) true)
  (Rendering|SetVisibility (Variables|Default|GetLantern2) (Variables|Default|GetLampBVisibility) true)
  (Rendering|SetVisibility (Variables|Default|GetLantern3) (Variables|Default|GetLampCVisbility) true)
  (Rendering|SetVisibility (Variables|Default|GetLantern4) (Variables|Default|GetLampDVisibility) true))